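; Base Blueprint for a playable human character that turns Enhanced Input actions into movement, jump, mouse and camera commands.
; On BeginPlay it adds the move, mouse and view mapping contexts to the player controller's subsystem.
; A small macro flags whether move input is active, zeroing the multiplier on release and otherwise choosing full or half speed from the run input.
; View actions toggle third-person view and adjust its camera distance.
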(event Input|EnhancedActionEvents|EnhancedInputActionINPA_Move
  (params (ActionValue :type Vector%202D%20Structure) (ElapsedSeconds :type Float%20%28double-precision%29) (TriggeredSeconds :type Float%20%28double-precision%29) (InputAction :type Input%20Action%20Object%20Reference :default "/Game/Main/Inputs/INPA_Move.INPA_Move"))
  (:Triggered
    (bind _isa (Utilities|WichExec :!label _label)
      (:Exec
        (Development|PrintString (Utilities|String|ToString(Boolean) _isa))
        (Class|CPPBaseCharacter|MovementInput ActionValue (Math|Float|SelectFloat (Math|Float|SelectFloat 1.0 0.5 (Input|EnhancedActionValues|GetINPA_MoveRun)) 0.0 _isa)))))
  (:Canceled
    (goto _label B))
  (:Completed
    (goto _label B)))

(event Input|EnhancedActionEvents|EnhancedInputActionINPA_Jump
  (params (ActionValue :type Boolean) (ElapsedSeconds :type Float%20%28double-precision%29) (TriggeredSeconds :type Float%20%28double-precision%29) (InputAction :type Input%20Action%20Object%20Reference :default "/Game/Main/Inputs/INPA_Jump.INPA_Jump"))
  (Class|CPPBaseCharacter|JumpInput))

(event Input|EnhancedActionEvents|EnhancedInputActionINPA_ViewChange
  (params (ActionValue :type Boolean) (ElapsedSeconds :type Float%20%28double-precision%29) (TriggeredSeconds :type Float%20%28double-precision%29) (InputAction :type Input%20Action%20Object%20Reference :default "/Game/Main/Inputs/INPA_ViewChange.INPA_ViewChange"))
  (Class|CPPBaseCharacter|ChangeCameraView (not (Variables|Default|GetisThridView)) false))

(event Input|EnhancedActionEvents|EnhancedInputActionINPA_View3PRegulate
  (params (ActionValue :type Float%20%28double-precision%29) (ElapsedSeconds :type Float%20%28double-precision%29) (TriggeredSeconds :type Float%20%28double-precision%29) (InputAction :type Input%20Action%20Object%20Reference :default "/Game/Main/Inputs/INPA_View3PRegulate.INPA_View3PRegulate"))
  (Class|CPPBaseCharacter|ChangeThridCameraDistance ActionValue))

(event Input|EnhancedActionEvents|EnhancedInputActionINPA_Mouse
  (params (ActionValue :type Vector%202D%20Structure) (ElapsedSeconds :type Float%20%28double-precision%29) (TriggeredSeconds :type Float%20%28double-precision%29) (InputAction :type Input%20Action%20Object%20Reference :default "/Game/Main/Inputs/INPA_Mouse.INPA_Mouse"))
  (:Triggered
    (Class|CPPBaseCharacter|MouseInput ActionValue :!label _label))
  (:Canceled
    (goto _label))
  (:Completed
    (goto _label)))

(event EventBeginPlay
  (|CallParentFunction)
  (Protected|InitVariables))

(fn ConstructionScript)

(fn InitVariables
  (Variables|Default|GetPlayerControllerBase
    (:then
      (Input|AddMappingContext (PlayerController|LocalPlayerSubsystems|GetEnhancedInputLocalPlayerSubsystem (Variables|Default|GetPlayerControllerBase)) "/Game/Main/Inputs/INPC_Move.INPC_Move" 0 "(bIgnoreAllPressedKeysUntilRelease=True,bForceImmediately=False,bNotifyUserSettings=False)")
      (Input|AddMappingContext (PlayerController|LocalPlayerSubsystems|GetEnhancedInputLocalPlayerSubsystem (Variables|Default|GetPlayerControllerBase)) "/Game/Main/Inputs/INPC_Mouse.INPC_Mouse" 0 "(bIgnoreAllPressedKeysUntilRelease=True,bForceImmediately=False,bNotifyUserSettings=False)")
      (Input|AddMappingContext (PlayerController|LocalPlayerSubsystems|GetEnhancedInputLocalPlayerSubsystem (Variables|Default|GetPlayerControllerBase)) "/Game/Main/Inputs/INPC_View.INPC_View" 0 "(bIgnoreAllPressedKeysUntilRelease=True,bForceImmediately=False,bNotifyUserSettings=False)"))
    (:else)))